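; Base weapon actor that the ThirdPersonCharacter can pick up in the world.
; A Sphere overlap shows a widget with the weapon name and [ F ] prompt, enables input and stores the character; leaving hides the prompt and clears CanPick.
; The Intrection action passes the weapon to the character's PickWeapon while CanPick is set, and CleanAll removes the sphere and prompt.
; The construction script writes the actor's own class into WeaponInfo.
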(event `self.Sphere.OnComponentBeginOverlap`
  (params (OverlappedComponent :type "PrimitiveComponent Object Reference") (OtherActor :type "Actor Object Reference") (OtherComp :type "PrimitiveComponent Object Reference") (OtherBodyIndex :type Integer) (bFromSweep :type Boolean) (SweepResult :type "HitResult Structure (by ref)"))
  (bind _asthird_person_character (cast `/Game/ThirdPersonBP/Blueprints/ThirdPersonCharacter` OtherActor))
  (set `self.PropleRef` _asthird_person_character)
  (`SceneComponent.SetVisibility` (`self.Widget`) true false)
  (set `self.CanPick?` true)
  (`self.EnableInput` (`GameplayStatics.GetPlayerController` 0))
  (set `/Game/GameUI/PickUpWB.ItemInfo` (`KismetTextLibrary.Conv_StringToText` (`KismetStringLibrary.Concat_StrStr` (`.Name_30_1770D59E4C79B3FA3CC6F0AC377E4F31` (break `/Game/GameBlueprints/BP_Weapons/WeaponInfo` (`self.WeaponInfo`))) "[ F ]")) (cast `/Game/GameUI/PickUpWB` (`WidgetComponent.GetUserWidgetObject` (`self.Widget`)) :!pure true)))

(event `self.Sphere.OnComponentEndOverlap`
  (params (OverlappedComponent :type "PrimitiveComponent Object Reference") (OtherActor :type "Actor Object Reference") (OtherComp :type "PrimitiveComponent Object Reference") (OtherBodyIndex :type Integer))
  (cast `/Game/ThirdPersonBP/Blueprints/ThirdPersonCharacter` OtherActor)
  (set `self.PropleRef` null)
  (`SceneComponent.SetVisibility` (`self.Widget`) false false)
  (set `self.CanPick?` false))

(event `InputAction|Intrection`
  (params (Key :type "Key Structure"))
  (:`Pressed`
    (if (`self.CanPick?`)
      (`/Game/ThirdPersonBP/Blueprints/ThirdPersonCharacter.PickWeapon` (`self.PropleRef`) self))))

(event `CleanAll`
  (`ActorComponent.K2_DestroyComponent` (`self.Sphere`))
  (`SceneComponent.SetVisibility` (`self.Widget`) false false))

(fn `UserConstructionScript`
  (bind (_weaponinfo_weapontype _weaponinfo_class _weaponinfo_image _weaponinfo_name _weaponinfo_damage _weaponinfo_range _weaponinfo_firerate _weaponinfo_curentammo _weaponinfo_maxammo _weaponinfo_unequipscoket) (break `/Game/GameBlueprints/BP_Weapons/WeaponInfo` (`self.WeaponInfo`)))
  (set `self.WeaponInfo` (make `/Game/GameBlueprints/BP_Weapons/WeaponInfo` _weaponinfo_weapontype (`GameplayStatics.GetObjectClass` self) _weaponinfo_image _weaponinfo_name _weaponinfo_damage _weaponinfo_range _weaponinfo_firerate _weaponinfo_curentammo _weaponinfo_maxammo _weaponinfo_unequipscoket)))